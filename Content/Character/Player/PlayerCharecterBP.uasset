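; PlayerCharecterBP is a player character Blueprint that handles basic movement and camera look from axis inputs.
; Forward and Right axes feed AddMovementInput along the controller actor's forward and right vectors.
; Mouse X and Y apply raw yaw and pitch deltas directly to the SpringArm's relative rotation, with no clamping and no change to control rotation.
; The construction script only calls its parent.
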(event `InputAxis|Forward`
  (params (AxisValue :type "Float (single-precision)"))
  (`self.AddMovementInput` (`self.GetActorForwardVector` (`self.GetController`)) AxisValue))

(event `InputAxis|Right`
  (params (AxisValue :type "Float (single-precision)"))
  (`self.AddMovementInput` (`self.GetActorRightVector` (`self.GetController`)) AxisValue))

(event `InputAxis|MouseAxisX`
  (params (AxisValue :type "Float (single-precision)"))
  (`SceneComponent.K2_AddRelativeRotation` (`self.SpringArm`) (`KismetMathLibrary.MakeRotator` 0.0 0.0 AxisValue) false false))

(event `InputAxis|MouseAxisY`
  (params (AxisValue :type "Float (single-precision)"))
  (`SceneComponent.K2_AddRelativeRotation` (`self.SpringArm`) (`KismetMathLibrary.MakeRotator` 0.0 AxisValue) false false))

(fn `UserConstructionScript`
  (`parent.UserConstructionScript`))